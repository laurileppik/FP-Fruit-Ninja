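; BP_FruitSpawner periodically spawns random fruit high above the world near the player for a slicing mechanic.
; A looping timer set on BeginPlay picks one of the first five fruit classes, spawns it at a fixed height and clears its IsSliced flag.
; X and Y offsets from the player use separate random angles, so spawns scatter within a square rather than on a ring.
; The SpawnFruit function is an empty stub.
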(event `self.ReceiveBeginPlay`
  (`KismetSystemLibrary.K2_SetTimerDelegate` (delegate `SpawnFruits`) 1.3 true))

(event `SpawnFruits`
  (bind _returnvalue (`KismetMathLibrary.DegreesToRadians` (`KismetMathLibrary.RandomFloatInRange` 0.0 360.0)))
  (bind _aspb_player (cast `/Game/Blueprints/PB_Player` (`GameplayStatics.GetPlayerPawn` 0)))
  (bind _output_get (set `self.RadiusOfFruitSpawn` 500.0))
  (bind (_returnvalue_x _returnvalue_y) (`KismetMathLibrary.BreakVector` (`self.K2_GetActorLocation` _aspb_player)))
  (bind _returnvalue_2 (`|SpawnActorFromClass` (`|GetArrayItem` (`self.FruitClassesArray`) (`KismetMathLibrary.RandomIntegerInRange` 0 4)) (`KismetMathLibrary.MakeTransform` (`KismetMathLibrary.MakeVector` (+ _returnvalue_x (* _output_get (`KismetMathLibrary.Cos` _returnvalue))) (+ _returnvalue_y (* _output_get (`KismetMathLibrary.Sin` _returnvalue))) 5500.0)) "AlwaysSpawn" "MultiplyWithRoot" null null))
  (bind _asfruit (cast `/Game/Blueprints/Fruit` _returnvalue_2))
  (set `/Game/Blueprints/Fruit.isSliced` false _asfruit))

(fn `SpawnFruit`)

(fn `UserConstructionScript`)