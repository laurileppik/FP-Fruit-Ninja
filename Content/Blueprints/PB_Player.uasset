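; Player Blueprint for a look-to-slice game: aiming at targets slices them for points, while aiming at a bomb ends the game.
; Mouse input turns the view, and BeginPlay adds a crosshair, teleports the player to a fixed start and resets Score.
; Every Tick, a camera line trace sends SliceMessage with a cutting plane to the hit actor.
; InteractInterface hits add score; BombInterface hits show the end screen with the score and pause the game.
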(event `InputVectorAxis|Mouse2D`
  (params (AxisValue :type "Vector Structure"))
  (`self.AddControllerYawInput` (.x AxisValue))
  (`self.AddControllerPitchInput` self (* (.y AxisValue) -1.0)))

(event `self.ReceiveBeginPlay`
  (bind _returnvalue (`PlayerState.GetPlayerController` (`GameplayStatics.GetPlayerState` 0)))
  (`|ExecutionSequence`
    (:`then_0`
      (bind _returnvalue_2 (`|GenericCreateObject` "/Game/WB_crosshair.WB_crosshair_C"))
      (`UserWidget.AddToViewport` _returnvalue_2 0))
    (:`then_1`
      (`self.K2_SetActorLocationAndRotation` (1540.0 2325.0 6022.012604) (struct :`Yaw` -90.0) false true)
      (set `PlayerController.bShowMouseCursor` false _returnvalue)
      (`WidgetBlueprintLibrary.SetInputMode_GameOnly` _returnvalue))
    (:`then_2`
      (set `self.score` 0))))

(event `self.ReceiveTick`
  (params (DeltaSeconds :type "Float (single-precision)"))
  (bind _returnvalue (`GameplayStatics.GetPlayerState` 0))
  (bind _camera (`self.Camera`))
  (bind _returnvalue_2 (`SceneComponent.K2_GetComponentLocation` _camera))
  (bind (_outhit _returnvalue_3) (`KismetSystemLibrary.LineTraceSingle` _returnvalue_2 (+ _returnvalue_2 (* (`SceneComponent.GetForwardVector` _camera) 1000000.0)) "TraceTypeQuery1"))
  (`|ExecutionSequence`
    (:`then_0`
      (bind (_bblockinghit _binitialoverlap _time _distance _location _impactpoint _normal _impactnormal _physmat _hitactor) (`GameplayStatics.BreakHitResult` _outhit))
      (message `/Game/Blueprints/Sliceable.Slice` _hitactor _location (0.0 0.2 1.0)))
    (:`then_1`
      (if _returnvalue_3
        (if (`KismetSystemLibrary.DoesImplementInterface` _hitactor "/Game/Blueprints/InteractInterface.InteractInterface_C")
          (bind _output_get (set `self.score` (+ 100 (`self.score`))))
          (`KismetSystemLibrary.PrintString` (`KismetStringLibrary.Conv_IntToString` _output_get))
          (elif (`KismetSystemLibrary.DoesImplementInterface` _hitactor "/Game/Blueprints/BombInterface.BombInterface_C")
            (`KismetSystemLibrary.PrintString` "BOMB")
            (bind _returnvalue_4 (`|CreateWidget` "/Game/Blueprints/EndScreenWidget.EndScreenWidget_C" null (`self.score`)))
            (`UserWidget.AddToViewport` _returnvalue_4 0)
            (set `PlayerController.bShowMouseCursor` true (`PlayerState.GetPlayerController` _returnvalue))
            (`WidgetBlueprintLibrary.SetInputMode_UIOnlyEx` (`PlayerState.GetPlayerController` _returnvalue) _returnvalue_4)
            (`GameplayStatics.SetGamePaused` true)))))))

(fn `UserConstructionScript`)