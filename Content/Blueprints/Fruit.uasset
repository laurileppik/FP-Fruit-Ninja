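; Fruit actor that is tossed upward with spin when spawned and can be sliced in two along a given plane.
; Construction copies the static mesh into a physics-simulated procedural mesh, destroys the original, then calls the launch event, which fires twice in total.
; Slice runs its cut once, creating a capped other half and applying impulses and spin to both pieces.
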(event `OnFruitSpawned`
  (`KismetSystemLibrary.PrintString` "fruit spawned")
  (`PrimitiveComponent.AddImpulse` (`self.ProceduralMesh`) (0.0 0.0 500.0) "None" true)
  (`PrimitiveComponent.AddAngularImpulseInDegrees` (`self.ProceduralMesh`) (200.0 100.0 50.0) "None" true))

(event `/Game/Blueprints/Sliceable.Slice`
  (params (PlanePosition :type "Vector Structure") (PlaneNormal :type "Vector Structure"))
  (bind _returnvalue (`KismetMathLibrary.MakeVector` 0.0 0.0 (.z (* PlaneNormal 1000))))
  (set `self.isSliced` true)
  (`/Engine/EditorBlueprintResources/StandardMacros.DoOnce` false
    (:`Completed`
      (bind _outotherhalfprocmesh (`KismetProceduralMeshLibrary.SliceProceduralMesh` (`self.ProceduralMesh`) PlanePosition PlaneNormal true "CreateNewSectionForCap"))
      (`PrimitiveComponent.SetSimulatePhysics` _outotherhalfprocmesh true)
      (`PrimitiveComponent.SetSimulatePhysics` (`self.ProceduralMesh`) true)
      (`PrimitiveComponent.AddAngularImpulseInDegrees` _outotherhalfprocmesh (0.0 300.0 0.0) "None" true)
      (`PrimitiveComponent.AddImpulse` _outotherhalfprocmesh _returnvalue "None" true)
      (`PrimitiveComponent.AddImpulse` (`self.ProceduralMesh`) _returnvalue "None" true)
      (`PrimitiveComponent.AddAngularImpulseInDegrees` (`self.ProceduralMesh`) (* PlaneNormal -200) "None" true))))

(fn `PrepareProceduralMesh`
  (bind _proceduralmesh (`self.ProceduralMesh`))
  (`KismetProceduralMeshLibrary.CopyProceduralMeshFromStaticMeshComponent` (`self.StaticMesh`) 0 _proceduralmesh true)
  (`PrimitiveComponent.SetSimulatePhysics` _proceduralmesh true)
  (`ActorComponent.K2_DestroyComponent` (`self.StaticMesh`))
  (`self.OnFruitSpawned`))

(fn `UserConstructionScript`
  (`self.PrepareProceduralMesh`)
  (`self.OnFruitSpawned`))